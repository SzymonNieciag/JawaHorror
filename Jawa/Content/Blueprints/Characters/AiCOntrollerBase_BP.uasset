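; Base AI controller Blueprint that assigns itself to team 1 on BeginPlay and reports perception changes as debug text.
; On each target perception update, it queries the AI Perception component for that actor's last sensed stimuli.
; Stimulus indices 0 and 1 are treated as sight and hearing, printing Polish visible/audible messages or their negations.
; It has no behavior response, and a node disabling sight is left unconnected.
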(event OnTargetPerceptionUpdated(AIPerceptionComponent)
  (params (Actor :type Actor%20Object%20Reference) (Stimulus :type AI%20Stimulus%20Structure))
  (bind _info (Class|AIPerceptionComponent|GetActorsPerception (Variables|Default|GetAIPerceptionComponent) Actor))
  (Utilities|FlowControl|Sequence
    (:then_0
      (if (.bsuccessfullysensed (Utilities|Array|Get(acopy) (.lastsensedstimuli _info)))
        (Development|PrintString "Widoczny")
        (else
          (Development|PrintString "Niewidoczny"))))
    (:then_1
      (if (.bsuccessfullysensed (Utilities|Array|Get(acopy) (.lastsensedstimuli _info) 1))
        (Development|PrintString "slyszalny")
        (else
          (Development|PrintString "nie slyszalny"))))))

(event EventBeginPlay
  (|CallParentFunction)
  (Class|AIControllerBase|SetGenericTeamId (Utilities|Struct|MakeGenericTeamId 1)))

(event EventTick
  (params (DeltaSeconds :type Float%20%28single-precision%29)))

(fn ConstructionScript)