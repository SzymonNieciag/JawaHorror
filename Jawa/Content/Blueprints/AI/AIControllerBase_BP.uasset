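; Base AI controller that sets its team ID, runs BT_Base and turns perception updates into character state changes.
; A successful first-sense stimulus sets the target, switches to Attacking and clears waypoints.
; Otherwise it spawns a waypoint at the second sense's stimulus, or at the first's last location while dropping the target, and switches to Searching.
; Each update then calls OnSenseAIUpdated.
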(event OnTargetPerceptionUpdated(AIPerceptionComponent)
  (params (Actor :type Actor%20Object%20Reference) (Stimulus :type AI%20Stimulus%20Structure))
  (bind _aicharacter (Variables|Default|GetAICharacter))
  (bind _aicharacter_2 (Variables|Default|GetAICharacter))
  (bind _aicharacter_3 (Variables|Default|GetAICharacter))
  (bind _waypoints (Variables|/Script/Jawa.AICharacter|GetWayPoints _aicharacter))
  (bind _info (Class|AIPerceptionComponent|GetActorsPerception (Variables|Default|GetAIPerceptionComponent) Actor))
  (if (.bsuccessfullysensed (Utilities|Array|Get(acopy) (.lastsensedstimuli _info)))
    (Variables|/Script/Jawa.AICharacter|SetTargetActor (Variables|Default|GetAICharacter) (.target _info))
    (Variables|/Script/Jawa.AICharacter|SetAICharacterState _aicharacter "Attacking")
    (for _array_element _waypoints
      (Actor|DestroyActor _array_element))
    (Utilities|Array|Clear _waypoints)
    (Default|CallOnSenseAIUpdated)
    (elif (.bsuccessfullysensed (Utilities|Array|Get(acopy) (.lastsensedstimuli _info) 1))
      (bind _returnvalue (Game|SpawnActorfromClass "/Game/Blueprints/AI/WayPoint_BP.WayPoint_BP_C" (Math|Transform|MakeTransform (.stimuluslocation (Utilities|Array|Get(acopy) (.lastsensedstimuli _info) 1)) "0, 0, 0" "1,1,1") "Undefined" _aicharacter_3 _aicharacter_3))
      (Utilities|Array|Add (Variables|/Script/Jawa.AICharacter|GetWayPoints (Variables|Default|GetAICharacter)) _returnvalue)
      (Variables|/Script/Jawa.AICharacter|SetAICharacterState (Variables|Default|GetAICharacter) "Searching")
      (Default|CallOnSenseAIUpdated)
      (else
        (bind _returnvalue_2 (Game|SpawnActorfromClass "/Game/Blueprints/AI/WayPoint_BP.WayPoint_BP_C" (Math|Transform|MakeTransform (.stimuluslocation (Utilities|Array|Get(acopy) (.lastsensedstimuli _info))) "0, 0, 0" "1,1,1") "Undefined" _aicharacter_2 _aicharacter_2))
        (Utilities|Array|Add (Variables|/Script/Jawa.AICharacter|GetWayPoints (Variables|Default|GetAICharacter)) _returnvalue_2)
        (Variables|/Script/Jawa.AICharacter|SetTargetActor (Variables|Default|GetAICharacter) 0)
        (Variables|/Script/Jawa.AICharacter|SetAICharacterState (Variables|Default|GetAICharacter) "Searching")
        (Default|CallOnSenseAIUpdated)))))

(event EventBeginPlay
  (|CallParentFunction)
  (Class|AIControllerBase|SetGenericTeamId (Utilities|Struct|MakeGenericTeamId 1))
  (AI|RunBehaviorTree "/Game/Blueprints/AI/BT_Base.BT_Base"))

(event EventTick
  (params (DeltaSeconds :type Float%20%28single-precision%29)))

(fn ConstructionScript)