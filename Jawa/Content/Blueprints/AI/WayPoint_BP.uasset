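; WayPoint_BP is an AI waypoint actor that marks a target for the AICharacter that owns it.
; When TargetAchieved fires, it removes itself from the owner's WayPoints array and sets that character to Idle if none remain.
; It then calls CallOnSenseAIUpdated on the owner's AIControllerBase and destroys itself, so each waypoint is single-use.
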(event EventBeginPlay)

(event Collision|EventActorBeginOverlap
  (params (OtherActor :type Actor%20Object%20Reference)))

(event EventTick
  (params (DeltaSeconds :type Float%20%28single-precision%29)))

(event EventTargetAchieved
  (bind _asaicharacter (Utilities|Casting|CastToAICharacter (Components|GetOwner)))
  (bind _output_get (Variables|Default|SetAICharacter _asaicharacter))
  (bind _asaicontroller_base (Utilities|Casting|CastToAIControllerBase (AI|GetAIController _asaicharacter)))
  (Variables|Default|SetAIControllerBase _asaicontroller_base)
  (Utilities|Array|RemoveItem (Variables|/Script/Jawa.AICharacter|GetWayPoints _output_get) self)
  (if (== (Utilities|Array|Length (Variables|/Script/Jawa.AICharacter|GetWayPoints (Variables|Default|GetAICharacter))) 0)
    (Variables|/Script/Jawa.AICharacter|SetAICharacterState (Variables|Default|GetAICharacter) "Idle"))
  (Default|CallOnSenseAIUpdated (Variables|Default|GetAIControllerBase))
  (Actor|DestroyActor))

(fn ConstructionScript)