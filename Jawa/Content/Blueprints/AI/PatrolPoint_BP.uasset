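; Patrol point actor for AI that draws a green debug area matching its box component's footprint.
; The construction script builds a flat procedural-mesh quad at zero height from the box's scaled X and Y extents, then applies a green debug material.
; The event graph holds only empty default events, so the Blueprint contains no patrol logic of its own.
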(event EventBeginPlay)

(event Collision|EventActorBeginOverlap
  (params (OtherActor :type Actor%20Object%20Reference)))

(event EventTick
  (params (DeltaSeconds :type Float%20%28single-precision%29)))

(fn ConstructionScript
  (bind _proceduralmesh (Variables|Default|GetProceduralMesh))
  (bind _boxcomponent (Variables|Default|GetBoxComponent))
  (bind _returnvalue (Components|Box|GetScaledBoxExtent _boxcomponent))
  (Class|ProceduralMeshComponent|CreateMeshSectionLinearColor _proceduralmesh 0 (Utilities|Array|MakeArray (Math|Vector|MakeVector (* (.x _returnvalue) -1.0) (* (.y _returnvalue) -1.0) 0.0) (Math|Vector|MakeVector (.x _returnvalue) (* (.y _returnvalue) -1.0) 0.0) (Math|Vector|MakeVector (* (.x _returnvalue) -1.0) (.y _returnvalue) 0.0) (Math|Vector|MakeVector (.x _returnvalue) (.y _returnvalue) 0.0)) (Utilities|Array|MakeArray 2 1 0 1 2 3) 0 (Utilities|Array|MakeArray "" "(X=1.000000,Y=0.000000)" "(X=0.000000,Y=1.000000)" "(X=1.000000,Y=1.000000)") 0 0 0 0 0 false)
  (Rendering|Material|SetMaterial _proceduralmesh 0 "/Game/Blueprints/AI/M_GreenDebug.M_GreenDebug"))